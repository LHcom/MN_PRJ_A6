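; BP_BDGameModeBase is a game mode that shows the lobby UI and handles the switch into gameplay input.
; BeginPlay adds WBP_LobyUI to the viewport, then after a short delay unpauses and sets UI-only input with a visible cursor.
; Tick polls the IsOnce flag; when true, it clears it, switches to game-only input, hides the cursor and starts the main 2D sound.
; Nothing in this graph sets IsOnce to true.
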(event `self.ReceiveBeginPlay`
  (bind _returnvalue (`GameplayStatics.GetPlayerController` 0))
  (bind _returnvalue_2 (`|CreateWidget` "/Game/UI/WBP_LobyUI.WBP_LobyUI_C"))
  (bind _output_get (set `self.LobyUiVar` _returnvalue_2))
  (`UserWidget.AddToViewport` _output_get 0)
  (`KismetSystemLibrary.Delay` 1.0)
  (`GameplayStatics.SetGamePaused` false)
  (`WidgetBlueprintLibrary.SetInputMode_UIOnlyEx` _returnvalue null)
  (set `PlayerController.bShowMouseCursor` true _returnvalue))

(event `self.ReceiveTick`
  (params (DeltaSeconds :type "Float (single-precision)"))
  (bind _returnvalue (`GameplayStatics.GetPlayerController` 0))
  (`|ExecutionSequence`
    (:`then_0`
      (if (== (`self.IsOnce`) true)
        (`WidgetBlueprintLibrary.SetInputMode_GameOnly` _returnvalue)
        (set `PlayerController.bShowMouseCursor` false _returnvalue)
        (set `self.IsOnce` false)
        (bind _returnvalue_2 (`GameplayStatics.SpawnSound2D` (`self.MainSound`) 1.0 1.0 0.0 null))
        (bind _output_get (set `self.MainAudioComp` _returnvalue_2))
        (`AudioComponent.Play` _output_get 0.0)))))

(fn `UserConstructionScript`)